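; BP_Button is a physical toggle button that a VRPawn presses by overlapping its box to start or stop the level's BP_Timer.
; On BeginPlay it caches the button's resting location, then each overlap eases the mesh down or back up with MoveComponentTo.
; Pressing sets a hardcoded start time on the timer found via GetActorOfClass and starts it, while releasing stops it.
; The trailing Delay after stopping gates nothing, so it provides no debounce.
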(event `self.ReceiveBeginPlay`
  (set `self.ButtonStart` (`SceneComponent.RelativeLocation` (`self.Button`))))

(event `self.Box.OnComponentBeginOverlap`
  (params (OverlappedComponent :type "PrimitiveComponent Object Reference") (OtherActor :type "Actor Object Reference") (OtherComp :type "PrimitiveComponent Object Reference") (OtherBodyIndex :type Integer) (bFromSweep :type Boolean) (SweepResult :type "HitResult Structure (by ref)"))
  (cast `/Game/VRTemplate/Blueprints/VRPawn` OtherActor)
  (if (`self.IsButtonPressed`)
    (`KismetSystemLibrary.MoveComponentTo` (`self.Button`) (`self.ButtonStart`) (struct) true)
    (set `self.IsButtonPressed` false)
    (bind _returnvalue (`GameplayStatics.GetActorOfClass` "/Game/Blueprint/BP_Timer.BP_Timer_C"))
    (`/Game/Blueprint/BP_Timer.StopTimer` _returnvalue)
    (`KismetSystemLibrary.Delay` 0.5)
    (else
      (`KismetSystemLibrary.MoveComponentTo` (`self.Button`) (- (`self.ButtonStart`) (0.0 0.0 5.0)) (struct) true)
      (set `self.IsButtonPressed` true)
      (bind _returnvalue_2 (`GameplayStatics.GetActorOfClass` "/Game/Blueprint/BP_Timer.BP_Timer_C"))
      (`/Game/Blueprint/BP_Timer.SetUpStartTimeFunc` _returnvalue_2 10.42069)
      (`/Game/Blueprint/BP_Timer.StartTimer` _returnvalue_2))))

(fn `UserConstructionScript`)