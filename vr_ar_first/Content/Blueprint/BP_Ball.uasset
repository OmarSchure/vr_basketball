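; Grabbable VR basketball that records how far from the hoop the player stands when releasing it.
; When its GrabComponent fires OnDropped, it looks up the VRPawn and a BP_Basket_Hoop found by class.
; It measures their horizontal distance, ignoring height, logs it with a German label and stores it in ThrowDistanceToHoop.
; The other events and the construction script are empty.
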(event `self.ReceiveBeginPlay`)

(event `self.GrabComponent.OnDropped`
  (bind _asvrpawn (cast `/Game/VRTemplate/Blueprints/VRPawn` (`GameplayStatics.GetPlayerPawn` 0)))
  (bind _returnvalue (`GameplayStatics.GetActorOfClass` "/Game/Blueprint/BP_Basket_Hoop.BP_Basket_Hoop_C"))
  (bind _returnvalue_2 (`KismetMathLibrary.Distance2D` (`KismetMathLibrary.MakeVector2D` (.x (`SceneComponent.K2_GetComponentLocation` (`Actor.RootComponent` _returnvalue))) (.y (`SceneComponent.K2_GetComponentLocation` (`Actor.RootComponent` _returnvalue)))) (`KismetMathLibrary.MakeVector2D` (.x (`SceneComponent.K2_GetComponentLocation` (`Actor.RootComponent` _asvrpawn))) (.y (`SceneComponent.K2_GetComponentLocation` (`Actor.RootComponent` _asvrpawn))))))
  (`KismetSystemLibrary.LogString` (`KismetStringLibrary.Concat_StrStr` "Der Abstand ist: " (`KismetStringLibrary.Conv_DoubleToString` _returnvalue_2)))
  (set `self.ThrowDistanceToHoop` _returnvalue_2))

(fn `UserConstructionScript`)