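; BP_Scoredisplay is a four-digit score display built from BP_7Segment child actors for units, tens, hundreds and thousands.
; Update_Score adds the incoming points to Score and splits the total into decimal digits with repeated division and modulo.
; CastAndUpdateSegment casts each child actor, sets its Digit and calls UpdateDigit.
; ResetScore runs on BeginPlay, zeroing Score and refreshing the display.
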(event `self.ReceiveBeginPlay`
  (`self.ResetScore`))

(event `Update_Score`
  (params (PlusScore :type Integer))
  (bind _output_get (set `self.Score` (+ PlusScore (`self.Score`))))
  (`|ExecutionSequence`
    (:`then_0`
      (`self.CastAndUpdateSegment` (`self.BP_7Segment_Units`) (mod _output_get 10)))
    (:`then_1`
      (bind _output_get_2 (set `self.ScoreInter` (/ _output_get 10)))
      (`self.CastAndUpdateSegment` (`self.BP_7Segment_Tens`) (mod _output_get_2 10)))
    (:`then_2`
      (bind _output_get_3 (set `self.ScoreInter` (/ _output_get_2 10)))
      (`self.CastAndUpdateSegment` (`self.BP_7Segment_Hundreds `) (mod _output_get_3 10)))
    (:`then_3`
      (bind _output_get_4 (set `self.ScoreInter` (/ _output_get_3 10)))
      (`self.CastAndUpdateSegment` (`self.BP_7Segment_Thousands`) (mod _output_get_4 10)))))

(event `ResetScore`
  (set `self.Score` 0)
  (`self.Update_Score` 0))

(fn `CastAndUpdateSegment`
  (params (Segment :type "ChildActorComponent Object Reference") (Digit :type Integer))
  (bind _asbp_7segment (cast `/Game/Blueprint/BP_7Segment` (`ChildActorComponent.ChildActor` Segment)))
  (set `/Game/Blueprint/BP_7Segment.Digit` Digit _asbp_7segment)
  (`/Game/Blueprint/BP_7Segment.Update_Digit` _asbp_7segment))

(fn `UserConstructionScript`)