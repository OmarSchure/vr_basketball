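; Basketball hoop actor that awards points when a BP_Ball passes downward through it.
; A Box overlap checks that the ball's Sphere has negative vertical velocity, so upward passes do not score, and logs the result.
; The ball's Points, plus one when its ThrowDistanceToHoop reaches the three-point range, go to UpdateScore on every BP_Scoredisplay found through GetAllActorsOfClass.
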(event `self.Box.OnComponentBeginOverlap`
  (params (OverlappedComponent :type "PrimitiveComponent Object Reference") (OtherActor :type "Actor Object Reference") (OtherComp :type "PrimitiveComponent Object Reference") (OtherBodyIndex :type Integer) (bFromSweep :type Boolean) (SweepResult :type "HitResult Structure (by ref)"))
  (bind _asbp_ball (cast `/Game/Blueprint/BP_Ball` OtherActor))
  (bind _returnvalue (`PrimitiveComponent.GetPhysicsLinearVelocity` (`/Game/Blueprint/BP_Ball.Sphere` _asbp_ball) "None"))
  (bind _returnvalue_2 (> 0.0 (.z _returnvalue)))
  (`KismetSystemLibrary.LogString` (`KismetStringLibrary.Concat_StrStr` "Z" (`KismetStringLibrary.Conv_BoolToString` _returnvalue_2)))
  (if _returnvalue_2
    (bind _outactors (`GameplayStatics.GetAllActorsOfClass` "/Game/Blueprint/BP_Scoredisplay.BP_Scoredisplay_C"))
    (if (>= (`/Game/Blueprint/BP_Ball.ThrowDistanceToHoop` _asbp_ball) (`self.3PointRange`))
      (bind _points (`/Game/Blueprint/BP_Ball.Points` _asbp_ball))
      (`/Game/Blueprint/BP_Scoredisplay.Update_Score` _outactors (+ _points 1))
      (else
        (`/Game/Blueprint/BP_Scoredisplay.Update_Score` _outactors _points)))))

(event `self.ReceiveActorBeginOverlap`
  (params (OtherActor :type "Actor Object Reference")))

(event `self.ReceiveTick`
  (params (DeltaSeconds :type "Float (single-precision)")))

(fn `UserConstructionScript`)