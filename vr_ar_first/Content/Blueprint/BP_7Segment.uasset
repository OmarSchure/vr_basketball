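; A seven-segment display actor that shows a single decimal digit by toggling the visibility of seven segment components, A through G.
; The Update_Digit event passes the Digit variable to a switch that selects the matching preset ActiveSegments array for values 0 to 9.
; DisplaSegments then applies each array entry to its segment through SetVisibilityOfSegment.
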(event `Update_Digit`
  (`self.ConvertDigitToBinArr` (`self.Digit`)))

(fn `ConvertDigitToBinArr`
  (params (Digit :type Integer))
  (switch `int` Digit
    (:`0`
      (`self.DisplaSegments` (`self.ActiveSegments0`)))
    (:`1`
      (`self.DisplaSegments` (`self.ActiveSegments1`)))
    (:`2`
      (`self.DisplaSegments` (`self.ActiveSegments2`)))
    (:`3`
      (`self.DisplaSegments` (`self.ActiveSegments3`)))
    (:`4`
      (`self.DisplaSegments` (`self.ActiveSegments4`)))
    (:`5`
      (`self.DisplaSegments` (`self.ActiveSegments5`)))
    (:`6`
      (`self.DisplaSegments` (`self.ActiveSegments6`)))
    (:`7`
      (`self.DisplaSegments` (`self.ActiveSegments7`)))
    (:`8`
      (`self.DisplaSegments` (`self.ActiveSegments8`)))
    (:`9`
      (`self.DisplaSegments` (`self.ActiveSegments9`)))))

(fn `DisplaSegments`
  (params (activeSegments :type "Array of Boolean"))
  (`|ExecutionSequence`
    (:`then_0`
      (`self.SetVisibilityOfSegment` (`self.a`) (`|GetArrayItem` activeSegments)))
    (:`then_1`
      (`self.SetVisibilityOfSegment` (`self.b`) (`|GetArrayItem` activeSegments 1)))
    (:`then_2`
      (`self.SetVisibilityOfSegment` (`self.c`) (`|GetArrayItem` activeSegments 2)))
    (:`then_3`
      (`self.SetVisibilityOfSegment` (`self.d`) (`|GetArrayItem` activeSegments 3)))
    (:`then_4`
      (`self.SetVisibilityOfSegment` (`self.e`) (`|GetArrayItem` activeSegments 4)))
    (:`then_5`
      (`self.SetVisibilityOfSegment` (`self.f`) (`|GetArrayItem` activeSegments 5)))
    (:`then_6`
      (`self.SetVisibilityOfSegment` (`self.g`) (`|GetArrayItem` activeSegments 6)))))

(fn `SetVisibilityOfSegment`
  (params (Object :type "StaticMeshComponent Object Reference") (Visibility :type Boolean))
  (`SceneComponent.SetVisibility` Object Visibility false))

(fn `UserConstructionScript`)