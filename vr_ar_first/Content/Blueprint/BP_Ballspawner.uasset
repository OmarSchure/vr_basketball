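; BP_Ballspawner is a spawner actor that keeps supplying BP_Ball actors at its Plane's location.
; It spawns one ball on BeginPlay, then another half a second after a BP_Ball ends overlap with the Spawn_Point component.
; An alternative sphere-overlap check for an empty spawn spot is left in the graph but never runs.
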(event `self.ReceiveBeginPlay`
  (`|SpawnActorFromClass` "/Game/Blueprint/BP_Ball.BP_Ball_C" (`KismetMathLibrary.Conv_VectorToTransform` (`SceneComponent.K2_GetComponentLocation` (`self.Plane`))) "Undefined" "MultiplyWithRoot" null null))

(event `self.ReceiveTick`
  (params (DeltaSeconds :type "Float (single-precision)")))

(event `self.Spawn_Point.OnComponentEndOverlap`
  (params (OverlappedComponent :type "PrimitiveComponent Object Reference") (OtherActor :type "Actor Object Reference") (OtherComp :type "PrimitiveComponent Object Reference") (OtherBodyIndex :type Integer))
  ; EventbasedSolution
  (cast `/Game/Blueprint/BP_Ball` OtherActor)
  (`KismetSystemLibrary.Delay` 0.5)
  (`|SpawnActorFromClass` "/Game/Blueprint/BP_Ball.BP_Ball_C" (`KismetMathLibrary.Conv_VectorToTransform` (`SceneComponent.K2_GetComponentLocation` (`self.Plane`))) "Undefined" "MultiplyWithRoot" null null))

(fn `UserConstructionScript`)