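; BP_Timer is a countdown timer actor that shows remaining time to the millisecond on five BP_7Segment child actors.
; While running, Tick subtracts delta time, then splits the millisecond count into digits by repeated modulo and division to update each segment.
; At zero it stops, plays a sound and fires a finished event dispatcher.
; BeginPlay loads the start time paused; StartTimer and StopTimer toggle the countdown.
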(event `StopTimer`
  (set `self.isRunning` false))

(event `StartTimer`
  (set `self.isRunning` true))

(event `self.ReceiveBeginPlay`
  (`self.SetUpStartTimeFunc` (`self.Starttime`)))

(event `self.ReceiveTick`
  (params (DeltaSeconds :type "Float (single-precision)"))
  (bind _returnvalue (- (`self.CurrentTime`) DeltaSeconds))
  (if (`self.isRunning`)
    (if (> _returnvalue 0.0)
      (bind _output_get (set `self.CurrentTime` _returnvalue))
      (bind _output_get_2 (set `self.TimeInMillieInt` (`KismetMathLibrary.FTrunc` (* _output_get 1000.0))))
      (`self.SetUpStartTime` _output_get_2)
      (else
        (set `self.isRunning` false)
        (set `self.CurrentTime` 0.0)
        (bind _output_get_3 (set `self.TimeInMillieInt` 0))
        (`self.SetUpStartTime` _output_get_3)
        (`GameplayStatics.PlaySoundAtLocation` "/Game/StarterContent/Audio/Collapse02.Collapse02" (`SceneComponent.K2_GetComponentLocation` (`self.DefaultSceneRoot`)) (struct) 1.0 1.0 0.0 null null null null)
        (`self.TimerIsFinished`)
        (`KismetSystemLibrary.PrintString` "Timer_BP: EventDispatcherCalled")))))

(fn `CalcNextDigit`
  (params (Segment :type "ChildActorComponent Object Reference") (DigitToBeDisplayed :type Integer))
  (returns (ForNextRot :type Integer))
  (bind _returnvalue (/ DigitToBeDisplayed 10))
  (`self.CastAndUpdateInTimerBP` Segment (mod _returnvalue 10))
  (return _returnvalue))

(fn `CastAndUpdateInTimerBP`
  (params (Segment :type "ChildActorComponent Object Reference") (Digit :type Integer))
  (bind _asbp_7segment (cast `/Game/Blueprint/BP_7Segment` (`ChildActorComponent.ChildActor` Segment)))
  (set `/Game/Blueprint/BP_7Segment.Digit` Digit _asbp_7segment)
  (`/Game/Blueprint/BP_7Segment.Update_Digit` _asbp_7segment))

(fn `SetUpStartTime`
  (params (MillieInTimeInt :type Integer))
  (`self.CastAndUpdateInTimerBP` (`self.Segment_Thousandths`) (mod MillieInTimeInt 10))
  (bind _fornextrot (`self.CalcNextDigit` (`self.Segment_Hundreths`) MillieInTimeInt))
  (bind _fornextrot_2 (`self.CalcNextDigit` (`self.Segment_Tenths`) _fornextrot))
  (bind _fornextrot_3 (`self.CalcNextDigit` (`self.Segment_Unit`) _fornextrot_2))
  (`self.CalcNextDigit` (`self.Segment_Tens`) _fornextrot_3))

(fn `SetUpStartTimeFunc`
  (params (StartTime :type "Float (double-precision)"))
  (`self.StopTimer`)
  (bind _output_get (set `self.CurrentTime` StartTime))
  (bind _output_get_2 (set `self.TimeInMillieInt` (`KismetMathLibrary.FTrunc` (* _output_get 1000.0))))
  (`self.SetUpStartTime` _output_get_2))

(fn `SubTime`
  (params (Digit :type Integer))
  (returns (Dig :type Integer))
  (return (- Digit 1)))

(fn `UserConstructionScript`)